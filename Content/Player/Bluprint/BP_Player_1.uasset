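; Player Blueprint that sets turn-in-place flags from look input and makes falls heavier than rises.
; While standing still, look input Y beyond a threshold sets TurningLeft or TurningRight through a helper; moving clears both.
; Both threshold else branches clear only TurningRight, so a right turn is immediately undone and TurningLeft can linger.
; Tick raises CharacterMovement gravity scale whenever vertical velocity is negative and restores it otherwise.
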(event `EnhancedInput|/Game/Player/Input/IA_PlayerInputLook`
  (params (ActionValue :type "Vector2D Structure") (ElapsedSeconds :type "Float (double-precision)") (TriggeredSeconds :type "Float (double-precision)") (InputAction :type "InputAction Object Reference" :default "/Game/Player/Input/IA_PlayerInputLook.IA_PlayerInputLook"))
  ;[1 1 1] TurnInPlaceBoolean
  (:`Triggered`
    (set `self.TurningValue` ActionValue_Y)
    (if (== (`KismetMathLibrary.VSize` (`self.GetVelocity`)) 0.0)
      (`|ExecutionSequence`
        (:`then_0`
          (if (> (`self.TurningValue`) 0.3)
            (`self.SetTurningLeft/Right ` true)
            (else
              (set `self.TurningRight` false))))
        (:`then_1`
          (if (< (`self.TurningValue`) -0.3)
            (`self.SetTurningLeft/Right ` false true)
            (else
              (set `self.TurningRight` false)))))
      (else
        (`self.SetTurningLeft/Right ` false)))))

(event `self.ReceiveBeginPlay`
  ;[1 1 1] TurnInPlaceBoolean
)

(event `self.ReceiveTick`
  (params (DeltaSeconds :type "Float (single-precision)"))
  (bind (_returnvalue_x _returnvalue_y _returnvalue_z) (`KismetMathLibrary.BreakVector` (`self.GetVelocity`)))
  ;[1 1 1] Gravity increase when the player rivh the highest point
  (if (> 0.0 _returnvalue_z)
    (set `CharacterMovementComponent.GravityScale` 1.5 (`self.CharacterMovement`))
    (else
      (set `CharacterMovementComponent.GravityScale` 1.0 (`self.CharacterMovement`)))))

(fn `UserConstructionScript`)