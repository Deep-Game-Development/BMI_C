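; Player character Blueprint for sword combat, with a blade slash projectile and a held block.
; Left click, gated by CanAttack and a forward trace tag check, fires the slash along camera rotation after a delay.
; PlaySwordAnimMontage attaches a temporary sword and sets that delay from montage length; both random branches play the same montage.
; Blocking loops its montage and disables attacks; other hooks trigger camera velocity calculation on landing and switch gravity scale.
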(event `self.OnLanded`
  (params (Hit :type "HitResult Structure (by ref)"))
  ;[0.05127 0.05127 0.05127] Call CalculateVelocity for CameraShake When Character Landed
  (`/Game/Player/Camera/BP_Camera.CalcVelocityDispatcher` (`self.BP_Camera`)))

(event `Key|LeftMouseButton`
  (params (Key :type "Key Structure"))
  (bind _returnvalue (`self.K2_GetActorLocation`))
  (bind (_returnvalue_location _returnvalue_rotation) (`KismetMathLibrary.BreakTransform` (`SceneComponent.K2_GetComponentToWorld` (`self.BP_Camera`))))
  (bind (_returnvalue_location_2 _returnvalue_rotation_2 _returnvalue_scale) (`KismetMathLibrary.BreakTransform` (`SceneComponent.K2_GetComponentToWorld` (`self.WhereThe BladeSlashSpawn `))))
  ;[0.07292 0.07292 0.07292 0.255] Spawn blade slash
  (:`Pressed`
    (if (`self.CanAttack`)
      (bind _outhit (`KismetSystemLibrary.SphereTraceSingleForObjects` _returnvalue (+ _returnvalue (* (`self.GetActorForwardVector`) 100.0)) 0.0 (`|MakeArray` "ObjectTypeQuery3" :!type "EObjectTypeQuery Enum")))
      (if (not (`KismetArrayLibrary.Array_Contains` (`Actor.Tags` (`.HitActor` (`GameplayStatics.BreakHitResult` _outhit)))))
        (`KismetSystemLibrary.Delay` (`self.SpawningProjectileDelay `))
        (bind _returnvalue_2 (`|SpawnActorFromClass` "/Game/Player/Projectiles/BP_BladeSlash.BP_BladeSlash_C" (`KismetMathLibrary.MakeTransform` _returnvalue_location_2 (`KismetMathLibrary.ComposeRotators` _returnvalue_rotation (struct :`Roll` 30.0)) _returnvalue_scale) "Undefined" "MultiplyWithRoot" null 1250.0 null))
        (`PrimitiveComponent.IgnoreActorWhenMoving` (`self.CapsuleComponent`) _returnvalue_2 true)))))

(event `EnhancedInput|/Game/Player/Input/IA_InputDefense`
  (params (ActionValue :type Boolean) (ElapsedSeconds :type "Float (double-precision)") (TriggeredSeconds :type "Float (double-precision)") (InputAction :type "InputAction Object Reference" :default "/Game/Player/Input/IA_InputDefense.IA_InputDefense"))
  ;[0.05208 0.05208 0.05208] Playing Defense Anim Montage
  (:`Started`
    (set `self.BBDefenseUp` true)
    (set `self.Can Play Defense montage ` true)
    (set `self.CanAttack` false)
    (if (`self.Can Play Defense montage `) :!label _label
      (`self.PlayAnimMontage` "/Game/Player/Animation/Defense/Standing_Block_Idle_Anim_Montage.Standing_Block_Idle_Anim_Montage")
      (`KismetSystemLibrary.Delay` 0.5)
      (goto _label)))
  (:`Completed`
    (set `self.BBDefenseUp` false)
    (set `self.Can Play Defense montage ` false)
    (set `self.CanAttack` true)
    (`self.StopAnimMontage` "/Game/Player/Animation/Defense/Standing_Block_Idle_Anim_Montage.Standing_Block_Idle_Anim_Montage")))

(fn `DestroySword`
  (`self.K2_DestroyActor` (`self.Sword`)))

(fn `GravityDicreaser`
  (set `CharacterMovementComponent.GravityScale` 1.0 (`self.CharacterMovement`)))

(fn `GravityIncreaser`
  (set `CharacterMovementComponent.GravityScale` 1.5 (`self.CharacterMovement`)))

(fn `PlaySwordAnimMontage`
  (bind _output_get (set `self.AttackIndex` (`KismetMathLibrary.RandomInteger` 2) :!label _label))
  (if (== _output_get (`self.LastValue `))
    (goto _label)
    (else
      (set `self.LastValue ` (`self.AttackIndex`))
      (switch `int` (`self.AttackIndex`)
        (:`0`
          (`/Engine/EditorBlueprintResources/StandardMacros.DoOnce` false :!label _label_2
            (:`Completed`
              (bind _returnvalue (`|SpawnActorFromClass` "/Game/Player/Mesh/Sword/Actor_Cube.Actor_Cube_C" (`self.GetTransform`) "Undefined" "MultiplyWithRoot" null null))
              (set `self.Sword` _returnvalue)
              (`self.K2_AttachToComponent` _returnvalue (`self.Mesh`) "hand_rSocket" "SnapToTarget" "SnapToTarget" "SnapToTarget" true)
              (bind _returnvalue_2 (`self.PlayAnimMontage` "/Game/Player/Animation/SwordAttacking/Sword_And_Shield_Slash1_Montage.Sword_And_Shield_Slash1_Montage"))
              (`KismetSystemLibrary.K2_SetTimer` null "DestroySword" _returnvalue_2)
              (set `self.SpawningProjectileDelay ` _returnvalue_2)
              (goto _label_2 :!via `Reset`))))
        (:`1`
          (`/Engine/EditorBlueprintResources/StandardMacros.DoOnce` false :!label _label_3
            (:`Completed`
              (bind _returnvalue_3 (`|SpawnActorFromClass` "/Game/Player/Mesh/Sword/Actor_Cube.Actor_Cube_C" (`self.GetTransform`) "Undefined" "MultiplyWithRoot" null null))
              (set `self.Sword` _returnvalue_3)
              (`self.K2_AttachToComponent` _returnvalue_3 (`self.Mesh`) "hand_rSocket" "SnapToTarget" "SnapToTarget" "SnapToTarget" true)
              (bind _returnvalue_4 (`self.PlayAnimMontage` "/Game/Player/Animation/SwordAttacking/Sword_And_Shield_Slash1_Montage.Sword_And_Shield_Slash1_Montage"))
              (`KismetSystemLibrary.K2_SetTimer` null "DestroySword" _returnvalue_4)
              (set `self.SpawningProjectileDelay ` _returnvalue_4)
              (goto _label_3 :!via `Reset`))))))))

(fn `UserConstructionScript`)